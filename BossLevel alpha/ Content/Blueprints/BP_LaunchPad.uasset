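; BP_LaunchPad is a mushroom launch pad that launches the third-person character vertically with a squish animation.
; From BeginPlay, a self-repeating 0.1-second delay loop line-traces upward from the root for Pawn objects instead of using overlap events.
; A hit on BP_ThirdPersonCharacter applies LaunchVelocity and plays a timeline that scales the mesh.
; A DoOnce, reset on each launch, lets that timeline reverse once to restore the shape.
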(event `self.ReceiveBeginPlay`
  (bind _defaultsceneroot (`self.DefaultSceneRoot`))
  (bind _outhit (`KismetSystemLibrary.LineTraceSingleForObjects` :`Start` (`SceneComponent.K2_GetComponentLocation` _defaultsceneroot) :`End` (+ (`SceneComponent.K2_GetComponentLocation` _defaultsceneroot) (`KismetMathLibrary.MakeVector` 0.0 0.0 (`self.Detection Height`))) :`ObjectTypes` (`|MakeArray` "ObjectTypeQuery3" :!type "EObjectTypeQuery Enum") :`DrawTime` 1.0 :!label _label))
  (`KismetSystemLibrary.Delay` 0.1)
  (`|ExecutionSequence`
    (:`then_0`
      (bind _asbp_third_person_character (cast `/Game/Blueprints/BP_ThirdPersonCharacter` (`.HitActor` (`GameplayStatics.BreakHitResult` _outhit))))
      (`Character.LaunchCharacter` _asbp_third_person_character (`KismetMathLibrary.MakeVector` 0.0 0.0 (`self.Launch Velocity`)) false false)
      (`|ExecutionSequence`
        (:`then_0`
          (bind (_direction _scale) (`Timeline|Squish Mushroom` :!label _label_2)
            (:`Update`
              (`SceneComponent.SetWorldScale3D` (`self.StaticMesh`) _scale))
            (:`Finished`
              (`/Engine/EditorBlueprintResources/StandardMacros.DoOnce` false :!label _label_3
                (:`Completed`
                  (goto _label_2 :!via `ReverseFromEnd`))))))
        (:`then_1`
          (goto _label_3 :!via `Reset`))))
    (:`then_1`
      (goto _label))))

(fn `UserConstructionScript`)