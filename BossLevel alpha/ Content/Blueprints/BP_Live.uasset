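; BP_Live is an extra-life pickup that spins in place until collected.
; BeginPlay randomly picks the spin direction, and Tick applies a fixed yaw step to the mesh each frame, without delta-time scaling.
; On collision overlap, it casts the overlapping actor's instigator to BP_ThirdPersonCharacter, adds one to that character's Lives and destroys itself.
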(event `self.ReceiveBeginPlay`
  (set `self.RotationSpeed` (select `bool` (`KismetMathLibrary.RandomBool`) :`false` 1.5 :`true` -1.5 :!type "Float (single-precision)")))

(event `self.ReceiveTick`
  (params (DeltaSeconds :type "Float (single-precision)"))
  (`SceneComponent.K2_AddRelativeRotation` (`self.StaticMesh`) (`KismetMathLibrary.MakeRotator` 0.0 0.0 (`self.RotationSpeed`)) false false))

(event `self.Collision.OnComponentBeginOverlap`
  (params (OverlappedComponent :type "PrimitiveComponent Object Reference") (OtherActor :type "Actor Object Reference") (OtherComp :type "PrimitiveComponent Object Reference") (OtherBodyIndex :type Integer) (bFromSweep :type Boolean) (SweepResult :type "HitResult Structure (by ref)"))
  (bind _asbp_third_person_character (cast `/Game/Blueprints/BP_ThirdPersonCharacter` (`self.GetInstigator` OtherActor)))
  (set `/Game/Blueprints/BP_ThirdPersonCharacter.Lives` (+ (`/Game/Blueprints/BP_ThirdPersonCharacter.Lives` _asbp_third_person_character) 1) _asbp_third_person_character)
  (`self.K2_DestroyActor`))

(fn `UserConstructionScript`)