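; BP_CollectableCoins is a spinning coin pickup that adds to the player's coin count.
; BeginPlay picks a random spin direction, and Tick yaws the mesh by a fixed amount each frame, not scaled by delta time.
; When PickUpRadius is overlapped, it casts the other actor's instigator to BP_ThirdPersonCharacter, adds CoinsToAdd to its Coins, prints the total and destroys itself.
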(event `self.ReceiveBeginPlay`
  (set `self.RotationSpeed` (select `bool` (`KismetMathLibrary.RandomBool`) :`false` 1.5 :`true` -1.5 :!type "Float (single-precision)")))

(event `self.ReceiveTick`
  (params (DeltaSeconds :type "Float (single-precision)"))
  (`SceneComponent.K2_AddRelativeRotation` (`self.Mesh`) (`KismetMathLibrary.MakeRotator` 0.0 0.0 (`self.RotationSpeed`)) false false))

(event `self.Pick Up Radius.OnComponentBeginOverlap`
  (params (OverlappedComponent :type "PrimitiveComponent Object Reference") (OtherActor :type "Actor Object Reference") (OtherComp :type "PrimitiveComponent Object Reference") (OtherBodyIndex :type Integer) (bFromSweep :type Boolean) (SweepResult :type "HitResult Structure (by ref)"))
  (bind _asbp_third_person_character (cast `/Game/Blueprints/BP_ThirdPersonCharacter` (`self.GetInstigator` OtherActor)))
  (bind _output_get (set `/Game/Blueprints/BP_ThirdPersonCharacter.Coins` (+ (`/Game/Blueprints/BP_ThirdPersonCharacter.Coins` _asbp_third_person_character) (`self.Coins To Add`)) _asbp_third_person_character))
  (`KismetSystemLibrary.PrintString` (`KismetStringLibrary.Conv_IntToString` _output_get))
  (`self.K2_DestroyActor`))

(fn `UserConstructionScript`)