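; BP_Checkpoint is a checkpoint actor that saves a respawn point when the third-person character enters its collision sphere.
; An overlap whose instigator is BP_ThirdPersonCharacter writes the RespawnLocation component's world transform to BP_GameInstance and sets its CheckpointOn flag.
; The save repeats on every overlap, while a DoOnce limits the HUD checkpoint animation and camera shutter sound to the first pass.
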(event `self.Sphere Collision.OnComponentBeginOverlap`
  (params (OverlappedComponent :type "PrimitiveComponent Object Reference") (OtherActor :type "Actor Object Reference") (OtherComp :type "PrimitiveComponent Object Reference") (OtherBodyIndex :type Integer) (bFromSweep :type Boolean) (SweepResult :type "HitResult Structure (by ref)"))
  (bind _asbp_third_person_character (cast `/Game/Blueprints/BP_ThirdPersonCharacter` (`self.GetInstigator` OtherActor)))
  (bind _asbp_game_instance (cast `/Game/Blueprints/BP_GameInstance` (`GameplayStatics.GetGameInstance`)))
  (set `/Game/Blueprints/BP_GameInstance.RespawnTransform` (`SceneComponent.K2_GetComponentToWorld` (`self.Respawn Location`)) _asbp_game_instance)
  (set `/Game/Blueprints/BP_GameInstance.CheckpointOn` true _asbp_game_instance)
  (`/Engine/EditorBlueprintResources/StandardMacros.DoOnce` false
    (:`Completed`
      (bind _hud_widget (`/Game/Blueprints/BP_ThirdPersonCharacter.HUD Widget` _asbp_third_person_character)
        (:`then`
          (`UserWidget.PlayAnimation` _hud_widget (`/Game/UI/Widgets/Widget_HUD.Checkpoint` _hud_widget) 0.0 1 "Forward" 1.0 false)
          (`GameplayStatics.PlaySound2D` "/Engine/VREditor/Sounds/UI/Camera_Shutter.Camera_Shutter" 1.0 1.0 0.0 null null))
        (:`else`)))))

(fn `UserConstructionScript`)