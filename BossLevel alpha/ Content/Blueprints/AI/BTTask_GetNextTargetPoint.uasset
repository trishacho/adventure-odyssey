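; Behavior tree task that advances an enemy's index into its list of target points.
; It casts the controlled pawn to BP_EnemyCharacter and compares the TargetPointIndex blackboard value with the length of the TargetPoints array on that enemy's TargetPointActor.
; While the index is below that length it writes back the incremented value and succeeds, otherwise it fails without resetting it.
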(event `self.ReceiveExecuteAI`
  (params (OwnerController :type "AIController Object Reference") (ControlledPawn :type "Pawn Object Reference"))
  (bind _asbp_enemy_character (cast `/Game/Blueprints/AI/BP_EnemyCharacter` ControlledPawn))
  (if (< (`BTFunctionLibrary.GetBlackboardValueAsInt` (`self.Target Point Index`)) (`KismetArrayLibrary.Array_Length` (`/Game/Blueprints/AI/BP_EnemyTargetPoints.Target Points` (`/Game/Blueprints/AI/BP_EnemyCharacter.Target Point Actor` _asbp_enemy_character))))
    (bind _result (`/Engine/EditorBlueprintResources/StandardMacros.IncrementInt` (`BTFunctionLibrary.GetBlackboardValueAsInt` (`self.Target Point Index`)))
      (:`  `
        (`BTFunctionLibrary.SetBlackboardValueAsInt` (`self.Target Point Index`) _result)
        (`self.FinishExecute` true)))
    (else
      (`self.FinishExecute` false))))