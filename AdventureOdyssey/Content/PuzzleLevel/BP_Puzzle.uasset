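; Sliding-tile puzzle actor that splits a texture across a square grid with one empty space.
; The construction script builds box slots and material-offset mesh tiles, optionally shuffling tile positions.
; Clicking a tile uses a sphere overlap to find an adjacent empty box, then a timeline slides it there with click events disabled.
; After each move, overlaps between tiles and their original slots determine the solved state, which is printed.
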(event `self.ReceiveBeginPlay`
  (for _array_element (`self.MeshesList`)
    (add `PrimitiveComponent.OnClicked` _array_element (delegate `MeshClicked`))))

(event `MeshClicked`
  (params (TouchedComponent :type "PrimitiveComponent Object Reference") (ButtonPressed :type "Key Structure" :default "None"))
  (bind _output_get (set `self.ClickedMesh` TouchedComponent))
  (add `PrimitiveComponent.OnClicked` _output_get (delegate `MeshClicked`))
  (bind _neighbors (`self.GetNeighbors`))
  (`self.GetMoveTo` _neighbors)
  (`/Engine/EditorBlueprintResources/StandardMacros.IsValid` (`self.MoveToTarget`)
    (:`Is Valid`
      (`self.MoveTo`))))

(event `MoveTo`
  (set `PlayerController.bEnableClickEvents` false (`GameplayStatics.GetPlayerController` 0))
  (set `self.MoveToStart` (`SceneComponent.RelativeLocation` (`self.ClickedMesh`)))
  (bind (_direction _newtrack_0) (`Timeline|Timeline` :!via `PlayFromStart`)
    (:`Update`
      (`SceneComponent.K2_SetRelativeLocation` (`self.ClickedMesh`) (`KismetMathLibrary.VLerp` (`self.MoveToStart`) (`SceneComponent.RelativeLocation` (`self.MoveToTarget`)) _newtrack_0) false false))
    (:`Finished`
      (set `PlayerController.bEnableClickEvents` true (`GameplayStatics.GetPlayerController` 0))
      (bind _solved (`self.IsSolved`))
      (`KismetSystemLibrary.PrintString` (`KismetStringLibrary.Conv_BoolToString` _solved)))))

(fn `GetMoveTo`
  (params (NeighborsList :type "Array of PrimitiveComponent Object Reference"))
  (set `self.MoveToTarget` null)
  (for _array_element NeighborsList
    (if (not (`PrimitiveComponent.IsOverlappingActor` _array_element self))
      (set `self.MoveToTarget` _array_element)))
  (return))

(fn `GetNeighbors`
  (returns (Neighbors :type "Array of PrimitiveComponent Object Reference"))
  (bind _outcomponents (`KismetSystemLibrary.SphereOverlapComponents` (`SceneComponent.K2_GetComponentLocation` (`self.ClickedMesh`)) (`self.MeshSize`) (`|MakeArray` "ObjectTypeQuery1" "ObjectTypeQuery2" :!type "EObjectTypeQuery Enum") "/Script/Engine.BoxComponent"))
  (return _outcomponents))

(fn `IsSolved`
  (returns (Solved :type Boolean))
  (locals (Solve :type Boolean :default true))
  (for (_array_element _array_index) (`self.MeshesList`)
    (if (not (`PrimitiveComponent.IsOverlappingComponent` _array_element (`|GetArrayItem` (`self.SpacesList`) _array_index)))
      (set `local.Solve` false)
      (break)))
  (return (`local.Solve`)))

(fn `ShufflePuzzle`
  (locals (Locations :type "Array of Vector Structure"))
  (bind _locations (`local.Locations`))
  (if (`self.Shuffle`)
    (for _array_element (`self.SpacesList`)
      (`KismetArrayLibrary.Array_Add` (`local.Locations`) (`SceneComponent.RelativeLocation` _array_element)))
    (`KismetArrayLibrary.Array_Shuffle` (`local.Locations`))
    (for _array_element_2 (`self.MeshesList`)
      (`SceneComponent.K2_SetRelativeLocation` _array_element_2 (`|GetArrayItem` _locations) false false)
      (`KismetArrayLibrary.Array_Remove` _locations))
    (return)
    (else
      (return))))

(fn `SpawnPuzzle`
  (bind _meshsize (`self.MeshSize`))
  (bind _spaceslist (`self.SpacesList`))
  (bind _mesheslist (`self.MeshesList`))
  (bind _meshsize_2 (`self.MeshSize`))
  (bind _returnvalue (- (`self.GridSize`) 1))
  (bind _returnvalue_2 (/ (`self.MeshSize`) 4.0))
  (bind _returnvalue_3 (- (`self.GridSize`) 1))
  (bind _returnvalue_4 (/ 1.0 (`KismetMathLibrary.Conv_IntToDouble` (`self.GridSize`))))
  (bind (_arrayindex _arrayelement) (`/Engine/EditorBlueprintResources/StandardMacros.ReverseForEachLoop` _spaceslist)
    (:`LoopBody`
      (`ActorComponent.K2_DestroyComponent` _arrayelement))
    (:`Completed`
      (`KismetArrayLibrary.Array_Clear` _spaceslist)
      (bind (_arrayindex_2 _arrayelement_2) (`/Engine/EditorBlueprintResources/StandardMacros.ReverseForEachLoop` _mesheslist)
        (:`LoopBody`
          (`ActorComponent.K2_DestroyComponent` _arrayelement_2))
        (:`Completed`
          (`KismetArrayLibrary.Array_Clear` _mesheslist)
          (for _index (range (+ _returnvalue 1))
            (set `self.YIndex` _index)
            (for _index_2 (range (+ _returnvalue 1))
              (set `self.XIndex` _index_2)
              (bind _returnvalue_5 (`AddComponent|NODE_AddBoxComponent-0` :`RelativeTransform` (`KismetMathLibrary.MakeTransform` (`KismetMathLibrary.MakeVector` (* (`self.XIndex`) _meshsize) (* (`self.YIndex`) _meshsize)))))
              (`BoxComponent.SetBoxExtent` _returnvalue_5 (`KismetMathLibrary.MakeVector` _returnvalue_2 _returnvalue_2 _returnvalue_2) true)
              (`KismetArrayLibrary.Array_Add` (`self.SpacesList`) _returnvalue_5)
              (if (not (and (== (`self.YIndex`) _returnvalue_3) (== _returnvalue_3 (`self.XIndex`))))
                (bind _returnvalue_6 (`AddComponent|NODE_AddStaticMeshComponent-0` :`RelativeTransform` (`KismetMathLibrary.MakeTransform` (`KismetMathLibrary.MakeVector` (* (`self.XIndex`) _meshsize_2) (* (`self.YIndex`) _meshsize_2)))))
                (`KismetArrayLibrary.Array_Add` (`self.MeshesList`) _returnvalue_6)
                (bind _returnvalue_7 (`PrimitiveComponent.CreateDynamicMaterialInstance` _returnvalue_6 0 "/Game/PuzzleLevel/M_PuzzleMaterial.M_PuzzleMaterial" "None"))
                (`MaterialInstanceDynamic.SetTextureParameterValue` _returnvalue_7 "PuzzleTexture" (`self.Texture`))
                (`MeshComponent.SetVectorParameterValueOnMaterials` _returnvalue_6 "TextureOffset2D" (`KismetMathLibrary.MakeVector` (* (`self.XIndex`) _returnvalue_4) (* (`self.YIndex`) _returnvalue_4) _returnvalue_4))))))))))

(fn `UserConstructionScript`
  (`self.SpawnPuzzle`)
  (`self.ShufflePuzzle`))