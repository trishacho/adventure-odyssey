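; Fire flower power-up for the Mario game that rises into place with a sound and powers up the player on pickup.
; On BeginPlay a timeline lerps it to TargetLocation, enabling collision when finished, while a morph-target blink replays after random retriggerable delays.
; When the player pawn overlaps PlayerDetection, it calls PowerUp on Mario_CharacterBP, spawns a particle burst at the player and destroys itself.
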(event `self.ReceiveBeginPlay`
  (`|ExecutionSequence`
    (:`then_0`
      (`PrimitiveComponent.SetCollisionEnabled` (`self.PlayerDetection`) "NoCollision"))
    (:`then_1`
      (bind (_direction _value) (`Timeline|BlinkTimeline` :!via `PlayFromStart` :!label _label)
        (:`Update`
          (`SkeletalMeshComponent.SetMorphTarget` (`self.Mesh`) "Blink" _value true)
          (`KismetSystemLibrary.RetriggerableDelay` (`KismetMathLibrary.RandomFloatInRange` 2.0 3.0))
          (goto _label :!via `PlayFromStart`))))
    (:`then_2`
      (bind (_direction_2 _value_2) (`Timeline|MoveUpTimeline`)
        (:`Update`
          (`self.K2_SetActorLocation` (`KismetMathLibrary.VLerp` (`self.K2_GetActorLocation`) (`self.TargetLocation`) _value_2)))
        (:`Finished`
          (`PrimitiveComponent.SetCollisionEnabled` (`self.CapsuleComponent`) "QueryAndPhysics")
          (`PrimitiveComponent.SetCollisionEnabled` (`self.PlayerDetection`) "QueryAndPhysics"))))
    (:`then_3`
      (`GameplayStatics.PlaySound2D` "/Game/Mario/SoundEffects/PowerUpAppears_SFX.PowerUpAppears_SFX" 1.0 1.0 0.0 null null))))

(event `self.PlayerDetection.OnComponentBeginOverlap`
  (params (OverlappedComponent :type "PrimitiveComponent Object Reference") (OtherActor :type "Actor Object Reference") (OtherComp :type "PrimitiveComponent Object Reference") (OtherBodyIndex :type Integer) (bFromSweep :type Boolean) (SweepResult :type "HitResult Structure (by ref)"))
  (if (== OtherActor (`Controller.K2_GetPawn` (`GameplayStatics.GetPlayerController` 0)))
    (bind _returnvalue (`GameplayStatics.GetActorOfClass` "/Game/Mario/Mario_CharacterBP.Mario_CharacterBP_C"))
    (`/Game/Mario/Mario_CharacterBP.PowerUp` _returnvalue)
    (`GameplayStatics.SpawnEmitterAtLocation` "/Game/FXVarietyPack/Particles/P_ky_explosion.P_ky_explosion" (`self.K2_GetActorLocation` (`Controller.K2_GetPawn` (`GameplayStatics.GetPlayerController` 0))) (struct) (0.7 0.7 0.7))
    (`self.K2_DestroyActor`)))

(fn `UserConstructionScript`)