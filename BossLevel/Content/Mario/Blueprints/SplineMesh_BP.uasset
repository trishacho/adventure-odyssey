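; Spline-driven Blueprint that builds a run of randomly varied meshes along its spline, with no active gameplay logic.
; The construction script divides the spline by SectionLength and adds a collision-enabled spline mesh component for each section.
; Each section randomly draws its mesh from the primary or secondary list, weighted toward primary.
; Start and end points follow the spline, with tangents clamped to the section length to fit each segment.
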(fn `UserConstructionScript`
  (bind _spline (`self.Spline`))
  (bind _spline_2 (`self.Spline`))
  (bind _returnvalue (select `bool` (`KismetMathLibrary.RandomBoolWithWeight` 0.8) :`false` (`self.SecondaryStaticMeshes`) :`true` (`self.PrimaryStaticMeshes`)))
  (for _index (range (+ (`KismetMathLibrary.FTrunc` (/ (`SplineComponent.GetSplineLength` (`self.Spline`)) (`self.SectionLength`))) 1))
    (bind _returnvalue_2 (`AddComponent|NODE_AddSplineMeshComponent-1`))
    (`StaticMeshComponent.SetStaticMesh` _returnvalue_2 (`|GetArrayItem` _returnvalue (`KismetMathLibrary.RandomIntegerInRange` 0 (- (`KismetArrayLibrary.Array_Length` _returnvalue) 1))))
    (`SplineMeshComponent.SetForwardAxis` _returnvalue_2 "X" true)
    (bind _returnvalue_3 (* (`self.SectionLength`) _index))
    (bind _returnvalue_4 (* (`self.SectionLength`) (+ _index 1)))
    (`SplineMeshComponent.SetStartAndEnd` _returnvalue_2 (`SplineComponent.GetLocationAtDistanceAlongSpline` _spline_2 _returnvalue_3 "Local") (`KismetMathLibrary.ClampVectorSize` (`SplineComponent.GetTangentAtDistanceAlongSpline` _spline_2 _returnvalue_3 "Local") 0.0 (`self.SectionLength`)) (`SplineComponent.GetLocationAtDistanceAlongSpline` _spline _returnvalue_4 "Local") (`KismetMathLibrary.ClampVectorSize` (`SplineComponent.GetTangentAtDistanceAlongSpline` _spline _returnvalue_4 "Local") 0.0 (`self.SectionLength`)) true)
    (`PrimitiveComponent.SetCollisionEnabled` _returnvalue_2 "QueryAndPhysics")))