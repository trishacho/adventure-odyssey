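; Mario floating ship actor that shuttles back and forth between the first two points of its spline.
; A timeline bobs the ship component vertically through a relative location lerp, independent of the root's travel.
; On BeginPlay it caches both points in world space, then endlessly moves the root to alternating ends, turning it 180 degrees in yaw between trips.
; Latent MoveComponentTo calls and random pauses pace the self-looping sequence.
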(event `self.ReceiveBeginPlay`
  (bind _spline (`self.Spline`))
  (bind _defaultsceneroot (`self.DefaultSceneRoot`))
  (bind (_relativerotation_roll _relativerotation_pitch _relativerotation_yaw) (`KismetMathLibrary.BreakRotator` (`SceneComponent.RelativeRotation` _defaultsceneroot)))
  (`|ExecutionSequence`
    (:`then_0`
      (bind (_direction _floatingvalue) (`Timeline|Floating`)
        (:`Update`
          (`SceneComponent.K2_SetRelativeLocation` (`self.FloatingShip`) (`KismetMathLibrary.VLerp` (0.0 0.0 0.0) (0.0 0.0 250.0) _floatingvalue) false false))))
    (:`then_1`
      (set `self.StartLoc` (`SplineComponent.GetLocationAtSplinePoint` _spline 0 "World"))
      (set `self.TargetLoc` (`SplineComponent.GetLocationAtSplinePoint` _spline 1 "World")))
    (:`then_2`
      (`KismetSystemLibrary.MoveComponentTo` (`self.DefaultSceneRoot`) (select `bool` (`self.Switch`) :`false` (`self.TargetLoc`) :`true` (`self.StartLoc`)) (`SceneComponent.RelativeRotation` (`self.DefaultSceneRoot`)) false false 30.0 :!label _label)
      (set `self.Switch` (not (`self.Switch`)))
      (`KismetSystemLibrary.RetriggerableDelay` (`KismetMathLibrary.RandomFloatInRange` 2.0 5.0))
      (`KismetSystemLibrary.MoveComponentTo` (`self.DefaultSceneRoot`) (`SceneComponent.RelativeLocation` _defaultsceneroot) (`KismetMathLibrary.MakeRotator` _relativerotation_roll _relativerotation_pitch (+ _relativerotation_yaw 180.0)) false false 5.0)
      (`KismetSystemLibrary.RetriggerableDelay` (`KismetMathLibrary.RandomFloatInRange` 2.0 5.0))
      (goto _label))))

(fn `UserConstructionScript`)