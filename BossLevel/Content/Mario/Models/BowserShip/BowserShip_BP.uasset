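; Bowser ship actor that wanders on its own between random points inside the bounds of MoveableAreaBox.
; On BeginPlay it picks a first target and snaps its yaw toward it.
; An endless latent loop then glides the root to the target with MoveComponentTo, pauses randomly, picks a new point, turns smoothly in yaw to face it, and pauses again before moving.
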(event `self.ReceiveBeginPlay`
  (bind (_origin _boxextent) (`self.GetActorBounds` (`self.MoveableAreaBox`) false false))
  (bind (_origin_2 _boxextent_2) (`self.GetActorBounds` (`self.MoveableAreaBox`) false false))
  (bind (_returnvalue_roll _returnvalue_pitch _returnvalue_yaw) (`KismetMathLibrary.BreakRotator` (`KismetMathLibrary.FindLookAtRotation` (`self.K2_GetActorLocation`) (`self.NextTargetLocation`))))
  (`|ExecutionSequence`
    (:`then_0`
      (bind _output_get (set `self.NextTargetLocation` (`KismetMathLibrary.RandomPointInBoundingBox` _origin _boxextent)))
      (bind (_returnvalue_roll_2 _returnvalue_pitch_2 _returnvalue_yaw_2) (`KismetMathLibrary.BreakRotator` (`KismetMathLibrary.FindLookAtRotation` (`self.K2_GetActorLocation`) _output_get)))
      (`self.K2_SetActorRotation` (`KismetMathLibrary.MakeRotator` 0.0 0.0 _returnvalue_yaw_2)))
    (:`then_1`
      (`KismetSystemLibrary.MoveComponentTo` (`self.DefaultSceneRoot`) (`self.NextTargetLocation`) (`SceneComponent.RelativeRotation` (`self.DefaultSceneRoot`)) false false 30.0 :!label _label)
      (`KismetSystemLibrary.RetriggerableDelay` (`KismetMathLibrary.RandomFloatInRange` 2.0 5.0))
      (set `self.NextTargetLocation` (`KismetMathLibrary.RandomPointInBoundingBox` _origin_2 _boxextent_2))
      (`KismetSystemLibrary.MoveComponentTo` (`self.DefaultSceneRoot`) (`SceneComponent.RelativeLocation` (`self.DefaultSceneRoot`)) (`KismetMathLibrary.MakeRotator` 0.0 0.0 _returnvalue_yaw) false false 3.0)
      (`KismetSystemLibrary.RetriggerableDelay` (`KismetMathLibrary.RandomFloatInRange` 2.0 5.0))
      (goto _label))))

(fn `UserConstructionScript`)