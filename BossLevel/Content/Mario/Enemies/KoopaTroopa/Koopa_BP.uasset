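; Koopa Troopa enemy that blinks at random intervals, walks forward and flips between two opposite facings when its wall trigger is overlapped.
; A player overlap from above spawns a Koopa shell and shares the ranged-hit defeat path (effects, score, player launch), while other player contact hurts Mario.
; Fire hits award score and animate Burnt then Dissolve parameters on dynamic materials before destroying the actor.
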(event `self.ReceiveBeginPlay`
  ;[0.2891 0 1] Begin play
  (bind (_direction _value) (`Timeline|Timeline` :!via `PlayFromStart` :!label _label)
    (:`Update`
      (`SkeletalMeshComponent.SetMorphTarget` (`self.Mesh`) "Blink" _value true))
    (:`Finished`
      (if (`self.Move?`)
        (`KismetSystemLibrary.Delay` (`KismetMathLibrary.RandomFloatInRange` 3.0 6.0))
        (goto _label :!via `PlayFromStart`)))))

(event `self.ReceiveTick`
  (params (DeltaSeconds :type "Float (single-precision)"))
  (bind (_returnvalue_roll _returnvalue_pitch _returnvalue_yaw) (`KismetMathLibrary.BreakRotator` (`self.GetControlRotation`)))
  ;[0.5937 1 0] Move
  (if (`self.Move?`)
    (`self.AddMovementInput` (`KismetMathLibrary.GetForwardVector` (`KismetMathLibrary.MakeRotator` 0.0 0.0 _returnvalue_yaw)))))

(event `self.WallDetection.OnComponentBeginOverlap`
  (params (OverlappedComponent :type "PrimitiveComponent Object Reference") (OtherActor :type "Actor Object Reference") (OtherComp :type "PrimitiveComponent Object Reference") (OtherBodyIndex :type Integer) (bFromSweep :type Boolean) (SweepResult :type "HitResult Structure (by ref)"))
  (bind _returnvalue (`self.K2_GetActorLocation`))
  (bind _capsulecomponent (`self.CapsuleComponent`))
  ;[0 1 0.3906] Wall Detection
  (if (and (!= OtherActor self) (!= OtherComp (`Controller.K2_GetPawn` (`GameplayStatics.GetPlayerController` 0))))
    (`PrimitiveComponent.SetCollisionEnabled` (`self.WallDetection`) "NoCollision")
    (`/Engine/EditorBlueprintResources/StandardMacros.FlipFlop`
      (:`A`
        (`KismetSystemLibrary.MoveComponentTo` _capsulecomponent _returnvalue (struct :`Yaw` 180.0) false false 0.15))
      (:`B`
        (`KismetSystemLibrary.MoveComponentTo` _capsulecomponent _returnvalue (struct) false false 0.15)))
    (`PrimitiveComponent.SetCollisionEnabled` (`self.WallDetection`) "QueryAndPhysics")))

(event `/Game/Mario/Enemies/Enemies_BPI.RangedHit`
  ;[1 0 0.4687] On player impact
  (`/Engine/EditorBlueprintResources/StandardMacros.DoOnce` false
    (:`Completed`
      (`GameplayStatics.PlaySound2D` "/Game/Mario/SoundEffects/Squash_SFX.Squash_SFX" 1.0 1.0 0.0 null null :!label _label_2)
      (`GameplayStatics.SpawnEmitterAtLocation` "/Game/Mario/Enemies/Goombas/P_ky_hit.P_ky_hit" (`SceneComponent.K2_GetComponentLocation` (`self.HitSpawnLoc`)) (struct) (0.5 0.5 0.5))
      (`/Game/Mario/Mario_CharacterBP.Change score/coins` (cast `/Game/Mario/Mario_CharacterBP` (`GameplayStatics.GetPlayerCharacter` 0) :!pure true) 100 0)
      (`ActorComponent.K2_DestroyComponent` (`self.WallDetection`))
      (`ActorComponent.K2_DestroyComponent` (`self.PlayerDetection`))
      (`GameplayStatics.SpawnEmitterAtLocation` "/Game/AdvancedMagicFX12/particles/P_ky_hit_shine.P_ky_hit_shine" (`SceneComponent.K2_GetComponentLocation` (`self.Mesh`)))
      (`self.LaunchCharacter` (`GameplayStatics.GetPlayerCharacter` 0) (0.0 0.0 250.0) false true)
      (`self.K2_DestroyActor`))))

(event `self.PlayerDetection.OnComponentBeginOverlap`
  (params (OverlappedComponent :type "PrimitiveComponent Object Reference") (OtherActor :type "Actor Object Reference") (OtherComp :type "PrimitiveComponent Object Reference") (OtherBodyIndex :type Integer) (bFromSweep :type Boolean) (SweepResult :type "HitResult Structure (by ref)"))
  (bind (_returnvalue_x _returnvalue_y _returnvalue_z) (`KismetMathLibrary.BreakVector` (`self.K2_GetActorLocation`)))
  (bind (_returnvalue_x_2 _returnvalue_y_2 _returnvalue_z_2) (`KismetMathLibrary.BreakVector` (`SceneComponent.K2_GetComponentLocation` (`Actor.RootComponent` (cast `Character` (`Controller.K2_GetPawn` (`GameplayStatics.GetPlayerController` 0)) :!pure true)))))
  ;[1 0 0.4687] On player impact
  (if (== OtherActor (`Controller.K2_GetPawn` (`GameplayStatics.GetPlayerController` 0)))
    (if (> (- _returnvalue_z_2 _returnvalue_z) 100.0)
      (`/Engine/EditorBlueprintResources/StandardMacros.DoOnce` false
        (:`Completed`
          (set `self.Move?` false)
          (`SkeletalMeshComponent.SetAnimation` (`self.Mesh`) null)
          (`|SpawnActorFromClass` "/Game/Mario/Enemies/KoopaTroopa/KoopaShell_BP.KoopaShell_BP_C" (`KismetMathLibrary.MakeTransform` (`SceneComponent.K2_GetComponentLocation` (`self.Mesh`))) "AlwaysSpawn" "OverrideRootScale" null null)
          (goto _label_2)))
      (else
        (`/Engine/EditorBlueprintResources/StandardMacros.DoOnce` false
          (:`Completed`
            (bind _asmario_character_bp (cast `/Game/Mario/Mario_CharacterBP` OtherActor))
            (`/Game/Mario/Mario_CharacterBP.On Hit` _asmario_character_bp (`KismetMathLibrary.GetDirectionUnitVector` (`self.K2_GetActorLocation`) (`self.K2_GetActorLocation` _asmario_character_bp)))))))))

(event `/Game/Mario/Enemies/Enemies_BPI.FireHit`
  (bind _mesh (`self.Mesh`))
  ;[0 0.2266 1] On hit
  (set `self.Move?` false)
  (`GameplayStatics.SpawnEmitterAtLocation` "/Game/AdvancedMagicFX12/particles/P_ky_hit_fire.P_ky_hit_fire" (`self.K2_GetActorLocation`))
  (`|ExecutionSequence`
    (:`then_0`
      (bind _returnvalue (`PrimitiveComponent.CreateDynamicMaterialInstance` _mesh 0 null "None"))
      (bind _returnvalue_2 (`PrimitiveComponent.CreateDynamicMaterialInstance` _mesh 1 null "None"))
      (bind _returnvalue_3 (`PrimitiveComponent.CreateDynamicMaterialInstance` _mesh 2 null "None"))
      (bind _returnvalue_4 (`PrimitiveComponent.CreateDynamicMaterialInstance` _mesh 3 null "None"))
      (bind _returnvalue_5 (`PrimitiveComponent.CreateDynamicMaterialInstance` _mesh 4 null "None"))
      (bind _returnvalue_6 (`PrimitiveComponent.CreateDynamicMaterialInstance` (`self.KoopaShell`) 0 null "None"))
      (`SkeletalMeshComponent.Stop` (`self.Mesh`))
      (bind (_direction _value) (`Timeline|Timeline_0`)
        (:`Update`
          (`MaterialInstanceDynamic.SetScalarParameterValue` _returnvalue_3 "Burnt" _value)
          (`MaterialInstanceDynamic.SetScalarParameterValue` _returnvalue_2 "Burnt" _value)
          (`MaterialInstanceDynamic.SetScalarParameterValue` _returnvalue "Burnt" _value)
          (`MaterialInstanceDynamic.SetScalarParameterValue` _returnvalue_5 "Burnt" _value)
          (`MaterialInstanceDynamic.SetScalarParameterValue` _returnvalue_4 "Burnt" _value)
          (`MaterialInstanceDynamic.SetScalarParameterValue` _returnvalue_6 "Burnt" _value))
        (:`Finished`
          (`KismetSystemLibrary.Delay` 0.5)
          (bind (_direction_2 _value_2) (`Timeline|Timeline_1`)
            (:`Update`
              (`MaterialInstanceDynamic.SetScalarParameterValue` _returnvalue_3 "Dissolve" _value_2)
              (`MaterialInstanceDynamic.SetScalarParameterValue` _returnvalue_2 "Dissolve" _value_2)
              (`MaterialInstanceDynamic.SetScalarParameterValue` _returnvalue "Dissolve" _value_2)
              (`MaterialInstanceDynamic.SetScalarParameterValue` _returnvalue_4 "Dissolve" _value_2)
              (`MaterialInstanceDynamic.SetScalarParameterValue` _returnvalue_5 "Dissolve" _value_2)
              (`MaterialInstanceDynamic.SetScalarParameterValue` _returnvalue_6 "Dissolve" _value_2))
            (:`Finished`
              (`self.K2_DestroyActor`))))))
    (:`then_1`
      (`/Game/Mario/Mario_CharacterBP.Change score/coins` (cast `/Game/Mario/Mario_CharacterBP` (`GameplayStatics.GetPlayerCharacter` 0) :!pure true) 100 0)
      (`GameplayStatics.PlaySound2D` "/Game/Mario/SoundEffects/Squash_SFX.Squash_SFX" 1.0 1.0 0.0 null null))))

(fn `UserConstructionScript`)