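; Koopa shell enemy character that starts sliding when the player stomps it and knocks out Goombas it touches.
; While moving, it walks forward along its control yaw each tick, and a wall trigger alternates the capsule between two opposite rotations.
; A player trigger uses height difference to pick a stomp, with score, effects and a bounce, or a one-time hit on Mario.
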(event `self.ReceiveTick`
  (params (DeltaSeconds :type "Float (single-precision)"))
  (bind (_returnvalue_roll _returnvalue_pitch _returnvalue_yaw) (`KismetMathLibrary.BreakRotator` (`self.GetControlRotation`)))
  ;[0 1 0.4375] Move
  (if (`self.Move?`)
    (`self.AddMovementInput` (`KismetMathLibrary.GetForwardVector` (`KismetMathLibrary.MakeRotator` 0.0 0.0 _returnvalue_yaw)))))

(event `self.WallDetection.OnComponentBeginOverlap`
  (params (OverlappedComponent :type "PrimitiveComponent Object Reference") (OtherActor :type "Actor Object Reference") (OtherComp :type "PrimitiveComponent Object Reference") (OtherBodyIndex :type Integer) (bFromSweep :type Boolean) (SweepResult :type "HitResult Structure (by ref)"))
  (bind _returnvalue (`self.K2_GetActorLocation`))
  (bind _capsulecomponent (`self.CapsuleComponent`))
  ;[1 0.9609 0] Wall detection
  (cast `Character` OtherActor
    (:`CastFailed`
      (if (`self.ActorHasTag` OtherActor "Ignore")
        _
        (elif (and (!= OtherActor self) (!= OtherComp (`Controller.K2_GetPawn` (`GameplayStatics.GetPlayerController` 0))))
          (`PrimitiveComponent.SetCollisionEnabled` (`self.WallDetection`) "NoCollision")
          (`/Engine/EditorBlueprintResources/StandardMacros.FlipFlop`
            (:`A`
              (`KismetSystemLibrary.MoveComponentTo` _capsulecomponent _returnvalue (struct :`Yaw` 180.0) false false 0.15))
            (:`B`
              (`KismetSystemLibrary.MoveComponentTo` _capsulecomponent _returnvalue (struct) false false 0.15)))
          (`PrimitiveComponent.SetCollisionEnabled` (`self.WallDetection`) "QueryAndPhysics"))))))

(event `self.PlayerDetection.OnComponentBeginOverlap`
  (params (OverlappedComponent :type "PrimitiveComponent Object Reference") (OtherActor :type "Actor Object Reference") (OtherComp :type "PrimitiveComponent Object Reference") (OtherBodyIndex :type Integer) (bFromSweep :type Boolean) (SweepResult :type "HitResult Structure (by ref)"))
  (bind (_returnvalue_x _returnvalue_y _returnvalue_z) (`KismetMathLibrary.BreakVector` (`self.K2_GetActorLocation`)))
  (bind (_returnvalue_x_2 _returnvalue_y_2 _returnvalue_z_2) (`KismetMathLibrary.BreakVector` (`SceneComponent.K2_GetComponentLocation` (`Actor.RootComponent` (cast `Character` (`Controller.K2_GetPawn` (`GameplayStatics.GetPlayerController` 0)) :!pure true)))))
  ;[0 1 0.2031] On enemy impact
  (if (== OtherActor (`Controller.K2_GetPawn` (`GameplayStatics.GetPlayerController` 0)))
    (if (> (- _returnvalue_z_2 _returnvalue_z) 80.0)
      (set `self.Move?` true)
      (`GameplayStatics.PlaySound2D` "/Game/Mario/SoundEffects/Squash_SFX.Squash_SFX" 1.0 1.0 0.0 null null)
      (`/Game/Mario/Mario_CharacterBP.Change score/coins` (cast `/Game/Mario/Mario_CharacterBP` (`GameplayStatics.GetPlayerCharacter` 0) :!pure true) 200 0)
      (`GameplayStatics.SpawnEmitterAtLocation` "/Game/AdvancedMagicFX12/particles/P_ky_hit_shine.P_ky_hit_shine" (`SceneComponent.K2_GetComponentLocation` (`self.Mesh`)))
      (`self.LaunchCharacter` (`GameplayStatics.GetPlayerCharacter` 0) (0.0 0.0 250.0) false true)
      (else
        (`/Engine/EditorBlueprintResources/StandardMacros.DoOnce` false
          (:`Completed`
            (bind _asmario_character_bp (cast `/Game/Mario/Mario_CharacterBP` OtherActor))
            (`/Game/Mario/Mario_CharacterBP.On Hit` _asmario_character_bp (`KismetMathLibrary.GetDirectionUnitVector` (`self.K2_GetActorLocation`) (`self.K2_GetActorLocation` _asmario_character_bp)))))))
    (else
      (bind _asgoomba_bp (cast `/Game/Mario/Enemies/Goombas/Goomba_BP` OtherActor))
      (`/Game/Mario/Enemies/Goombas/Goomba_BP.GoombaHit` _asgoomba_bp))))

(fn `UserConstructionScript`)