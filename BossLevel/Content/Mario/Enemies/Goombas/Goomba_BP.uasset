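; Goomba enemy that walks forward and flips 180 degrees when its wall trigger overlaps anything but the player.
; A falling player high enough over the hit trigger squashes it via timeline and bounces up, while the player trigger damages Mario once.
; Generic and ranged hits kill it immediately; fire hits run burn-then-dissolve timelines on dynamic materials.
; Every kill awards score through Mario_CharacterBP.
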(event `self.ReceiveTick`
  (params (DeltaSeconds :type "Float (single-precision)"))
  (bind (_returnvalue_roll _returnvalue_pitch _returnvalue_yaw) (`KismetMathLibrary.BreakRotator` (`self.GetControlRotation`)))
  ;[0 0.5078 1] Move
  (if (`self.Move?`)
    (`self.AddMovementInput` (`KismetMathLibrary.GetForwardVector` (`KismetMathLibrary.MakeRotator` 0.0 0.0 _returnvalue_yaw)))))

(event `self.WallDetection.OnComponentBeginOverlap`
  (params (OverlappedComponent :type "PrimitiveComponent Object Reference") (OtherActor :type "Actor Object Reference") (OtherComp :type "PrimitiveComponent Object Reference") (OtherBodyIndex :type Integer) (bFromSweep :type Boolean) (SweepResult :type "HitResult Structure (by ref)"))
  (bind _returnvalue (`self.K2_GetActorLocation`))
  (bind _walldetection (`self.WallDetection`))
  (bind _capsulecomponent (`self.CapsuleComponent`))
  ;[1 0 0.9141] Wall Detection
  (if (and (!= OtherActor self) (!= OtherActor (`Controller.K2_GetPawn` (`GameplayStatics.GetPlayerController` 0))))
    (`PrimitiveComponent.SetCollisionEnabled` (`self.WallDetection`) "NoCollision")
    (if (`self.Move?`)
      (`/Engine/EditorBlueprintResources/StandardMacros.FlipFlop`
        (:`A`
          (`KismetSystemLibrary.MoveComponentTo` _capsulecomponent _returnvalue (struct :`Yaw` 180.0) false false 0.15))
        (:`B`
          (`KismetSystemLibrary.MoveComponentTo` _capsulecomponent _returnvalue (struct) false false 0.15)))
      (`/Engine/EditorBlueprintResources/StandardMacros.IsValid` _walldetection
        (:`Is Valid`
          (`PrimitiveComponent.SetCollisionEnabled` _walldetection "QueryAndPhysics"))))))

(event `self.HitDetection.OnComponentBeginOverlap`
  (params (OverlappedComponent :type "PrimitiveComponent Object Reference") (OtherActor :type "Actor Object Reference") (OtherComp :type "PrimitiveComponent Object Reference") (OtherBodyIndex :type Integer) (bFromSweep :type Boolean) (SweepResult :type "HitResult Structure (by ref)"))
  (bind (_returnvalue_x _returnvalue_y _returnvalue_z) (`KismetMathLibrary.BreakVector` (`self.K2_GetActorLocation`)))
  (bind _returnvalue (`Controller.K2_GetPawn` (`GameplayStatics.GetPlayerController` 0)))
  (bind _ascharacter (cast `Character` _returnvalue :!pure true))
  (bind _charactermovement (`Character.CharacterMovement` _ascharacter))
  (bind (_returnvalue_x_2 _returnvalue_y_2 _returnvalue_z_2) (`KismetMathLibrary.BreakVector` (`SceneComponent.K2_GetComponentLocation` (`Actor.RootComponent` _ascharacter))))
  (bind (_velocity_x _velocity_y _velocity_z) (`KismetMathLibrary.BreakVector` (`MovementComponent.Velocity` _charactermovement)))
  ;[1 0.6328 0] Hit detection
  (if (== OtherActor _returnvalue)
    (if (and (`NavMovementComponent.IsFalling` _charactermovement) (< _velocity_z 0.0))
      (if (> (- _returnvalue_z_2 _returnvalue_z) 70.0)
        (`/Engine/EditorBlueprintResources/StandardMacros.DoOnce` false
          (:`Completed`
            (set `self.Move?` false)
            (`SkeletalMeshComponent.SetAnimation` (`self.Mesh`) null)
            (`GameplayStatics.PlaySound2D` "/Game/Mario/SoundEffects/Squash_SFX.Squash_SFX" 1.0 1.0 0.0 null null)
            (`GameplayStatics.SpawnEmitterAtLocation` "/Game/Mario/Enemies/Goombas/P_ky_hit.P_ky_hit" (`SceneComponent.K2_GetComponentLocation` (`self.HitDetection`)) (struct) (0.5 0.5 0.5))
            (`self.LaunchCharacter` (`GameplayStatics.GetPlayerCharacter` 0) (0.0 0.0 250.0) false true)
            (`/Game/Mario/Mario_CharacterBP.Change score/coins` (cast `/Game/Mario/Mario_CharacterBP` (`GameplayStatics.GetPlayerCharacter` 0) :!pure true) 100 0)
            (`ActorComponent.K2_DestroyComponent` (`self.WallDetection`))
            (`ActorComponent.K2_DestroyComponent` (`self.PlayerDetection`))
            (bind (_direction _value) (`Timeline|SquashGoomba`)
              (:`Update`
                (`SceneComponent.SetRelativeScale3D` (`self.CapsuleComponent`) (`KismetMathLibrary.VLerp` (1.0 1.0 1.0) (1.0 1.0 0.2) _value)))
              (:`Finished`
                (`GameplayStatics.SpawnEmitterAtLocation` "/Game/AdvancedMagicFX12/particles/P_ky_hit_shine.P_ky_hit_shine" (`SceneComponent.K2_GetComponentLocation` (`self.Mesh`)) :!label _label)
                (`self.K2_DestroyActor`)))))))))

(event `GoombaHit`
  ;[1 0.6328 0] Hit detection
  (`/Game/Mario/Mario_CharacterBP.Change score/coins` (cast `/Game/Mario/Mario_CharacterBP` (`GameplayStatics.GetPlayerCharacter` 0) :!pure true) 100 0 :!label _label_2)
  (`ActorComponent.K2_DestroyComponent` (`self.WallDetection`))
  (`ActorComponent.K2_DestroyComponent` (`self.PlayerDetection`))
  (`GameplayStatics.PlaySoundAtLocation` "/Game/Mario/SoundEffects/Squash_SFX.Squash_SFX" (`self.K2_GetActorLocation`) (struct) 1.0 1.0 0.0 null null null null)
  (goto _label))

(event `/Game/Mario/Enemies/Enemies_BPI.RangedHit`
  ;[1 0.6328 0] Hit detection
  (`/Engine/EditorBlueprintResources/StandardMacros.DoOnce` false
    (:`Completed`
      (goto _label_2))))

(event `self.PlayerDetection.OnComponentBeginOverlap`
  (params (OverlappedComponent :type "PrimitiveComponent Object Reference") (OtherActor :type "Actor Object Reference") (OtherComp :type "PrimitiveComponent Object Reference") (OtherBodyIndex :type Integer) (bFromSweep :type Boolean) (SweepResult :type "HitResult Structure (by ref)"))
  ;[0.5 0 1] On player impact
  (if (== OtherActor (`Controller.K2_GetPawn` (`GameplayStatics.GetPlayerController` 0)))
    (`/Engine/EditorBlueprintResources/StandardMacros.DoOnce` false
      (:`Completed`
        (bind _asmario_character_bp (cast `/Game/Mario/Mario_CharacterBP` OtherActor))
        (`/Game/Mario/Mario_CharacterBP.On Hit` _asmario_character_bp (`KismetMathLibrary.GetDirectionUnitVector` (`self.K2_GetActorLocation`) (`self.K2_GetActorLocation` _asmario_character_bp)))))))

(event `/Game/Mario/Enemies/Enemies_BPI.FireHit`
  (bind _mesh (`self.Mesh`))
  ;[0 0.2266 1] On hit
  (set `self.Move?` false)
  (`GameplayStatics.SpawnEmitterAtLocation` "/Game/AdvancedMagicFX12/particles/P_ky_hit_fire.P_ky_hit_fire" (`self.K2_GetActorLocation`))
  (`|ExecutionSequence`
    (:`then_0`
      (bind _returnvalue (`PrimitiveComponent.CreateDynamicMaterialInstance` _mesh 0 null "None"))
      (bind _returnvalue_2 (`PrimitiveComponent.CreateDynamicMaterialInstance` _mesh 1 null "None"))
      (bind _returnvalue_3 (`PrimitiveComponent.CreateDynamicMaterialInstance` _mesh 2 null "None"))
      (bind _returnvalue_4 (`PrimitiveComponent.CreateDynamicMaterialInstance` _mesh 3 null "None"))
      (`SkeletalMeshComponent.SetAnimationMode` (`self.Mesh`) "AnimationBlueprint")
      (bind (_direction _value) (`Timeline|MaterialBurn`)
        (:`Update`
          (`MaterialInstanceDynamic.SetScalarParameterValue` _returnvalue_3 "Burnt" _value)
          (`MaterialInstanceDynamic.SetScalarParameterValue` _returnvalue_2 "Burnt" _value)
          (`MaterialInstanceDynamic.SetScalarParameterValue` _returnvalue "Burnt" _value))
        (:`Finished`
          (`KismetSystemLibrary.Delay` 0.5)
          (bind (_direction_2 _value_2) (`Timeline|MaterialDissolve`)
            (:`Update`
              (`MaterialInstanceDynamic.SetScalarParameterValue` _returnvalue_3 "Dissolve" _value_2)
              (`MaterialInstanceDynamic.SetScalarParameterValue` _returnvalue_2 "Dissolve" _value_2)
              (`MaterialInstanceDynamic.SetScalarParameterValue` _returnvalue "Dissolve" _value_2)
              (`MaterialInstanceDynamic.SetScalarParameterValue` _returnvalue_4 "Dissolve" _value_2))
            (:`Finished`
              (`self.K2_DestroyActor`))))))
    (:`then_1`
      (`/Game/Mario/Mario_CharacterBP.Change score/coins` (cast `/Game/Mario/Mario_CharacterBP` (`GameplayStatics.GetPlayerCharacter` 0) :!pure true) 100 0)
      (`GameplayStatics.PlaySound2D` "/Game/Mario/SoundEffects/Squash_SFX.Squash_SFX" 1.0 1.0 0.0 null null))))

(fn `UserConstructionScript`)