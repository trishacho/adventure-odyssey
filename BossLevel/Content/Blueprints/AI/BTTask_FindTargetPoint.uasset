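; Behavior tree task that picks the enemy's next target point from its assigned TargetPointActor.
; It reads TargetPointIndex from the blackboard, transforms that TargetPoints entry from the actor's local space to world space, and writes it to the TargetPoint key.
; When the index is out of range, it resets the index to zero and fails; it does not advance the index itself.
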(event `self.ReceiveExecuteAI`
  (params (OwnerController :type "AIController Object Reference") (ControlledPawn :type "Pawn Object Reference"))
  (bind _returnvalue (`BTFunctionLibrary.GetBlackboardValueAsInt` (`self.Target Point Index`)))
  (bind _asbp_enemy_character (cast `/Game/Blueprints/AI/BP_EnemyCharacter` ControlledPawn))
  (bind _target_point_actor (`/Game/Blueprints/AI/BP_EnemyCharacter.Target Point Actor` _asbp_enemy_character))
  (bind _target_points (`/Game/Blueprints/AI/BP_EnemyTargetPoints.Target Points` _target_point_actor))
  (if (> (`KismetArrayLibrary.Array_Length` _target_points) _returnvalue)
    (`BTFunctionLibrary.SetBlackboardValueAsVector` (`self.Target Point`) (`KismetMathLibrary.TransformLocation` (`Actor.GetTransform` _target_point_actor) (`|GetArrayItem` _target_points _returnvalue)))
    (`self.FinishExecute` true)
    (else
      (`BTFunctionLibrary.SetBlackboardValueAsInt` (`self.Target Point Index`))
      (`self.FinishExecute` false))))