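; BP_Spikes is a hazard that deals repeated damage to the third-person character while it overlaps the spikes' Box.
; On overlap begin, if the instigator's health is above zero, it sets TouchingSpikes, then subtracts DamageSubtracted and calls the character's death check.
; A Delay loop repeats this every DurationBeforeDamage while the flag holds, without rechecking health, and end overlap clears the flag.
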(event `self.Box.OnComponentBeginOverlap`
  (params (OverlappedComponent :type "PrimitiveComponent Object Reference") (OtherActor :type "Actor Object Reference") (OtherComp :type "PrimitiveComponent Object Reference") (OtherBodyIndex :type Integer) (bFromSweep :type Boolean) (SweepResult :type "HitResult Structure (by ref)"))
  ;[1 1 1] Touching Spikes
  (bind _asbp_third_person_character (cast `/Game/Blueprints/BP_ThirdPersonCharacter` (`self.GetInstigator` OtherActor)))
  (if (not (<= (`/Game/Blueprints/BP_ThirdPersonCharacter.CurrentHealth` _asbp_third_person_character) 0.0))
    (set `self.TouchingSpikes` true)
    (`/Game/Blueprints/BP_ThirdPersonCharacter.Subtract Health` _asbp_third_person_character (`self.Damage Subtracted`) :!label _label)
    (`/Game/Blueprints/BP_ThirdPersonCharacter.Check For Death` _asbp_third_person_character)
    (`KismetSystemLibrary.Delay` (`self.Duration Before Damage`))
    (if (`self.TouchingSpikes`)
      (goto _label))))

(event `self.Box.OnComponentEndOverlap`
  (params (OverlappedComponent :type "PrimitiveComponent Object Reference") (OtherActor :type "Actor Object Reference") (OtherComp :type "PrimitiveComponent Object Reference") (OtherBodyIndex :type Integer))
  ;[1 1 1] Not touching spikes anymore
  (cast `/Game/Blueprints/BP_ThirdPersonCharacter` (`self.GetInstigator` OtherActor))
  (set `self.TouchingSpikes` false))

(fn `UserConstructionScript`)